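; WorkerBuyerPlate is an actor Blueprint that visually reflects a worker's upgrade level; it contains no purchase logic of its own.
; Every Tick it reads WorkerLevel from its WorkerUpgrader reference and, when that is above zero, casts the upgrader's TargetWorker to Worker.
; It then sets that worker's Crystal1 relative scale, widening X and Y linearly with level while Z stays fixed.
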(event EventBeginPlay)

(event Collision|EventActorBeginOverlap
  (params (OtherActor :type Actor%20Object%20Reference)))

(event EventTick
  (params (DeltaSeconds :type Float%20%28single-precision%29))
  (bind _workerupgrader (Variables|Default|GetWorkerUpgrader))
  (bind _workerlevel (Variables|/Script/ENG02_Challenge1.WorkerUpgrader|GetWorkerLevel _workerupgrader))
  (bind _returnvalue (Math|Conversions|ToFloat(Integer) _workerlevel))
  (bind _returnvalue_2 (* _returnvalue 0.1))
  (bind _returnvalue_3 (+ _returnvalue_2 0.2))
  (Math|Integer|CompareInt _workerlevel
    (:>
      (bind _asworker (Utilities|Casting|CastToWorker (Variables|/Script/ENG02_Challenge1.WorkerUpgrader|GettargetWorker _workerupgrader)))
      (Transformation|SetRelativeScale3D (Variables|/Game/Blueprints/Worker.Worker_C|GetCrystal_1 _asworker) (Math|Vector|MakeVector _returnvalue_3 _returnvalue_3 0.3)))))

(fn ConstructionScript)