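; Worker Blueprint for a resource-gathering character that shows what it is carrying.
; Each tick it reads the WorkeMoverCollector component's dropoff and stone-collecting flags.
; While heading to dropoff, it shows a rock pile mesh for stone or a tree log mesh otherwise, and hides both at other times.
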(event EventBeginPlay)

(event Collision|EventActorBeginOverlap
  (params (OtherActor :type Actor%20Object%20Reference)))

(event EventTick
  (params (DeltaSeconds :type Float%20%28single-precision%29))
  (bind _workemovercollector (Variables|Default|GetWorkeMoverCollector))
  (bind _iscollectingstone (Variables|/Script/ENG02_Challenge1.WorkeMoverCollector|GetisCollectingStone _workemovercollector))
  (bind _isgoingtodropoff (Variables|/Script/ENG02_Challenge1.WorkeMoverCollector|GetisGoingToDropoff _workemovercollector))
  (Rendering|SetVisibility (Variables|Default|GetSM_RockPilesBigB) (and _isgoingtodropoff _iscollectingstone) false)
  (Rendering|SetVisibility (Variables|Default|GetSM_TreeLogDarkB) (and _isgoingtodropoff (not _iscollectingstone)) false))

(fn ConstructionScript)